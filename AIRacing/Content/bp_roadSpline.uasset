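; Spline-based road actor that builds a drivable track and reports how a car sits relative to it.
; The construction script tiles colliding, shadowless spline meshes along the spline, with section length scaled by actor X scale and tangents clamped to it.
; BeginPlay adds tangent-aligned child actors at PointRingSectionLength intervals.
; Helper functions return a bp_car's heading angle against the track tangent and a location's distance from the spline.
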(event EventBeginPlay
  (bind _pointringsectionlength (Variables|Default|GetpointRingSectionLength))
  (for _index (range 0 (Math|Float|Truncate (/ (Spline|GetSplineLength (Variables|Default|GetSpline)) _pointringsectionlength)))
    (bind (_position _tangent) (CallFunction|GetStartPos/Tangent _index _pointringsectionlength))
    (AddComponent|AddChildActorComponent false (Math|Transform|MakeTransform _position (Math|Conversions|RotationFromXVector _tangent) "1.000000,1.000000,1.000000"))))

(event EventTick
  (params (DeltaSeconds :type Float%20%28single-precision%29)))

(fn ConstructionScript
  (Variables|Default|SetsectionLength (* (.x (Transformation|GetActorScale3D)) 5e+01))
  (Utilities|FlowControl|Sequence
    (:then_0
      ;[0.15 0.15 0.15 0.5] spawn road meshes
      (for _index (range 0 (Math|Float|Truncate (/ (Spline|GetSplineLength (Variables|Default|GetSpline)) (Variables|Default|GetsectionLength))))
        (bind _returnvalue (AddComponent|AddSplineMeshComponent false))
        (Components|StaticMesh|SetStaticMesh _returnvalue (Variables|Default|GetsplineMesh))
        (SplineMesh|SetForwardAxis _returnvalue "X" true)
        (bind (_position _tangent) (CallFunction|GetStartPos/Tangent _index (Variables|Default|GetsectionLength)))
        (bind (_position_2 _tangent_2) (CallFunction|GetEndPos/Tangent _index))
        (SplineMesh|SetStartandEnd _returnvalue _position _tangent _position_2 _tangent_2 true :!class /Script/Engine.SplineMeshComponent)
        (Collision|SetCollisionEnabled _returnvalue "QueryAndPhysics")
        (Collision|SetCollisionResponsetoAllChannels _returnvalue "ECR_Block")
        (Rendering|SetCastShadow _returnvalue false)))))

(fn GetStartPos/Tangent
  (params (index :type Integer) (section%20length :type Float%20%28double-precision%29))
  (bind _returnvalue (* index section%20length))
  (bind _spline (Variables|Default|GetSpline))
  (return (Spline|GetLocationatDistanceAlongSpline _spline _returnvalue "Local") (Math|Vector|ClampVectorSize (Spline|GetTangentatDistanceAlongSpline _spline _returnvalue "Local") 0.0 section%20length)))

(fn GetEndPos/Tangent
  (params (index :type Integer))
  (bind _returnvalue (+ index 1))
  (bind _spline (Variables|Default|GetSpline))
  (bind _sectionlength (Variables|Default|GetsectionLength))
  (bind _returnvalue_2 (* _returnvalue _sectionlength))
  (return (Spline|GetLocationatDistanceAlongSpline _spline _returnvalue_2 "Local") (Math|Vector|ClampVectorSize (Spline|GetTangentatDistanceAlongSpline _spline _returnvalue_2 "Local") 0.0 (Variables|Default|GetsectionLength))))

(fn GetStartPosRingPoints/Tangent
  (params (index :type Integer))
  (bind _spline (Variables|Default|GetSpline))
  (return (Spline|GetLocationatSplinePoint _spline index "Local") (Math|Vector|ClampVectorSize (Spline|GetTangentatSplinePoint _spline index "Local") 0.0 (Variables|Default|GetsectionLength))))

(fn GetEndPosRingPoints/Tangent
  (params (index :type Integer))
  (bind _returnvalue (+ index 1))
  (bind _spline (Variables|Default|GetSpline))
  (return (Spline|GetLocationatSplinePoint _spline _returnvalue "Local") (Math|Vector|ClampVectorSize (Spline|GetTangentatSplinePoint _spline _returnvalue "Local") 0.0 (Variables|Default|GetsectionLength))))

(fn GetAngletoTrack
  (params (car :type Car%20Object%20Reference))
  (bind _spline (Variables|Default|GetSpline))
  (bind _asbp_car (Utilities|Casting|CastTobp_car car))
  (return (Math|Trig|RadiansToDegrees (Math|Trig|Acos(Degrees) (/ (Math|Vector|DotProduct (Math|Vector|Normalize (Spline|GetTangentatDistanceAlongSpline _spline (Class|SplineComponent|GetDistanceAlongSplineatLocation _spline (.location (Transformation|GetActorTransform _asbp_car)) "World") "World")) (Math|Vector|Normalize (Transformation|GetActorForwardVector _asbp_car))) (* (Math|Vector|VectorLength (Math|Vector|Normalize (Spline|GetTangentatDistanceAlongSpline _spline (Class|SplineComponent|GetDistanceAlongSplineatLocation _spline (.location (Transformation|GetActorTransform _asbp_car)) "World") "World"))) (Math|Vector|VectorLength (Math|Vector|Normalize (Transformation|GetActorForwardVector _asbp_car)))))))))

(fn GetDistancefromTrackatLocation
  (params (Location :type Vector))
  (bind _spline (Variables|Default|GetSpline))
  (return (Math|Vector|Distance(Vector) (Spline|GetLocationatDistanceAlongSpline _spline (Class|SplineComponent|GetDistanceAlongSplineatLocation _spline Location "World") "World") Location)))