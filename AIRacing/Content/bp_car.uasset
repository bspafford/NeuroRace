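; Self-driving car that feeds track sensor data to a neural network and scores its driving fitness.
; While alive, each tick passes five forward-fan raycast distances, angle to the road spline and speed to CallFeedForward.
; Straying too far from the spline destroys the car; R resets its transform and velocity.
; CalcFitness adds scaled average speed to an inverted spline-position percentage, without counting laps.
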(event EventSpawnSkidMarks
  (params (skidMarks :type Boolean))
  (Class|NiagaraComponent|SetVariableBool (Variables|Default|GetskidMarksRight) "shouldSpawn" skidMarks)
  (Class|NiagaraComponent|SetVariableBool (Variables|Default|GetskidMarksLeft) "shouldSpawn" skidMarks))

(event EventBpBeginPlay
  (Variables|fitness|SetspawnTime 0.0)
  (bind _ascar_score (Utilities|Casting|CastTocarScore (UserInterface|GetWidget (Variables|Default|GetWidget))))
  (Variables|/Game/carScore.carScore_C|Setcar _ascar_score self))

(event EventBpDestroyCar
  (Utilities|FlowControl|Delay 0.2)
  (Actor|DestroyActor))

(event EventBpTick
  (params (deltaTime :type Float%20%28single-precision%29))
  (bind _returnvalue (Transformation|GetActorLocation))
  (Utilities|FlowControl|Sequence
    (:then_0
      (if (Variables|Default|GetbAlive)
        (Variables|Default|SetspeedSum (+ (Math|Vector|VectorLength (Transformation|GetVelocity)) (Variables|Default|GetspeedSum)))
        (Variables|Default|SetspeedNum (+ (Variables|Default|GetspeedNum) 1))
        (Variables|fitness|SetspawnTime (+ deltaTime (Variables|fitness|GetspawnTime)))
        ;[0.15 0.15 0.15 0.5] angle
        (bind _returnvalue_2 (Actor|GetActorOfClass "/Game/bp_roadSpline.bp_roadSpline_C"))
        (bind _returnvalue_3 (Default|GetAngletoTrack _returnvalue_2 self))
        ;[0.15 0.15 0.15 0.5] distance sensors
        (Utilities|Array|Clear (Variables|Default|Getdistances))
        (for _index (range 0 4)
          (bind _outhit (Collision|LineTraceByChannel (- _returnvalue "0.000000,0.000000,-100.000000") (- (+ _returnvalue (* 1e+04 (Math|Vector|RotateVector (Transformation|GetActorForwardVector) (Math|Rotator|MakeRotator 0.0 0.0 (- (* _index 45.0) 9e+01))))) "0.000000,0.000000,-100.000000") "TraceTypeQuery1" false 0 "None"))
          (Utilities|Array|Add (Variables|Default|Getdistances) (.distance _outhit)))
        (Class|Car|CallFeedForward (Variables|Default|Getdistances) _returnvalue_3 (Math|Vector|VectorLength (Transformation|GetVelocity)))))
    (:then_1
      (bind _returnvalue_4 (Actor|GetActorOfClass "/Game/bp_roadSpline.bp_roadSpline_C"))
      (bind _distance (Default|GetDistancefromTrackatLocation _returnvalue_4 (Transformation|GetActorLocation)))
      (if (>= _distance 2e+02)
        (Class|Car|DestroyCar)))))

(event Input|KeyboardEvents|R
  (params (Key :type Key%20Structure :default "None"))
  (:Pressed
    (Transformation|SetActorLocation "-1360.000000,-10.000000,31.490001" false false)
    (Variables|/Script/Engine.MovementComponent|SetVelocity (Variables|Character|GetCharacterMovement) "0, 0, 0")
    (Transformation|SetActorRotation "0.000000,180.000000,0.000000")))

(fn ConstructionScript)

(fn CalcFitness
  (bind _returnvalue (Actor|GetActorOfClass "/Game/bp_roadSpline.bp_roadSpline_C"))
  (Variables|Fitness|SetlapNum_0 (* (/ (- (Spline|GetSplineLength (Variables|/Game/bp_roadSpline.bp_roadSpline_C|GetSpline _returnvalue)) (Class|SplineComponent|GetDistanceAlongSplineatLocation (Variables|/Game/bp_roadSpline.bp_roadSpline_C|GetSpline _returnvalue) (Transformation|GetActorLocation) "World")) (Spline|GetSplineLength (Variables|/Game/bp_roadSpline.bp_roadSpline_C|GetSpline _returnvalue))) 1e+02))
  (Variables|Fitness|SetavgSpeed (/ (Variables|Default|GetspeedSum) (Variables|Default|GetspeedNum)))
  (return (+ 0.0 (/ (Variables|Fitness|GetavgSpeed) 75.0) (Variables|Fitness|GetlapNum_0))))