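; Orthographic camera actor that follows the front car in a race along a road spline.
; BeginPlay sets a fixed ortho width and rotation.
; Each tick it gathers every Bp_car, ranks them with SortCarList against the Bp_roadSpline spline, and interpolates its X and Y toward the first car in the sorted list.
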(event EventBeginPlay
  (Class|CameraComponent|SetOrthoWidth (Variables|Default|Getcamera) 1.5e+03)
  (Transformation|SetActorRotation "-90.000000,0.000000,180.000000"))

(event EventTick
  (params (DeltaSeconds :type Float%20%28single-precision%29))
  (bind _furthestcarlist (Variables|Default|GetfurthestCarList))
  (bind _returnvalue (Actor|GetActorOfClass "/Game/bp_roadSpline.bp_roadSpline_C"))
  (bind _outactors (Actor|GetAllActorsOfClass "/Game/bp_car.bp_car_C"))
  (Utilities|Array|Clear (Variables|Default|GetfurthestCarList))
  (for _array_element _outactors
    (Utilities|Array|Add (Variables|Default|GetfurthestCarList) _array_element))
  (if (!= (Utilities|Array|Length _furthestcarlist) 0)
    (bind _returnvalue_2 (Class|Camera|SortCarList _furthestcarlist (Variables|/Game/bp_roadSpline.bp_roadSpline_C|GetSpline _returnvalue)))
    (Transformation|SetActorLocation (Math|Vector|MakeVector (.x (Math|Interpolation|VInterpTo (Transformation|GetActorLocation) (Transformation|GetActorLocation (Utilities|Array|Get(acopy) _returnvalue_2)) (Utilities|Time|GetWorldDeltaSeconds) 1e+01)) (.y (Math|Interpolation|VInterpTo (Transformation|GetActorLocation) (Transformation|GetActorLocation (Utilities|Array|Get(acopy) _returnvalue_2)) (Utilities|Time|GetWorldDeltaSeconds) 1e+01)) 0.0) false false)))

(fn ConstructionScript)